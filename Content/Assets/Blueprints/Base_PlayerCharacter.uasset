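; Base player character for a Pac-Man-style level, tracking pickups and enemies and creating the HUD.
; Each pickup shrinks the collectible list; emptying it or dying triggers LevelEnd, which recolors the player, slows time and shows the matching result widget.
; Power pickups make living enemies flee and become killable until a retriggerable delay restores their chase.
; Left Shift boosts speed and jump height with a particle effect.
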(event `self.ReceiveBeginPlay`
  (`|ExecutionSequence`
    (:`then_0`
      (set `self.PlayerController` (`GameplayStatics.GetPlayerController` 0)))
    (:`then_1`
      (bind _outactors (`GameplayStatics.GetAllActorsOfClass` "/Game/Assets/Blueprints/Base_Pickup.Base_Pickup_C"))
      (bind _output_get (set `self.AllCollectiblesList` _outactors))
      (set `self.TotalPickups` (`KismetArrayLibrary.Array_Length` _output_get)))
    (:`then_2`
      (bind _outactors_2 (`GameplayStatics.GetAllActorsOfClass` "/Game/Assets/Blueprints/Base_Enemy.Base_Enemy_C"))
      (set `self.EnemiesList` _outactors_2))
    (:`then_3`
      (bind _returnvalue (`|CreateWidget` "/Game/Assets/Blueprints/Widgets/Widget_UI.Widget_UI_C" null self))
      (bind _output_get_2 (set `self.HUD` _returnvalue))
      (`UserWidget.AddToViewport` _output_get_2 0))))

(event `self.CharacterDeath`
  (set `self.IsCharacterAlive?` false)
  (set `self.CanCharacterDie?` false)
  (`self.LevelEnd`)
  (`GameplayStatics.PlaySound2D` "/Game/Assets/Blueprints/Audio/HeroDeath.HeroDeath" 1.0 1.0 0.0 null null))

(event `LevelEnd`
  (bind _enemy (`self.Enemy`))
  (`CharacterMovementComponent.DisableMovement` (`self.CharacterMovement`))
  (`self.ChangeColors` (select `bool` (`self.IsCharacterAlive?`) :`false` (select `bool` (`KismetSystemLibrary.IsValid` _enemy) :`false` (struct :`A` 1.0) :`true` (`/Game/Assets/Blueprints/MasterCharacter.Color` _enemy)) :`true` (struct :`R` 1.0 :`G` 1.0 :`B` 1.0 :`A` 1.0)))
  (`GameplayStatics.SetGlobalTimeDilation` 0.3)
  (`KismetSystemLibrary.Delay` 0.2)
  (if (`self.IsCharacterAlive?`)
    (if (== (`self.NextLevel`) "0")
      (bind _returnvalue (`|CreateWidget` "/Game/Assets/Blueprints/Widgets/Widget_GameCompleted.Widget_GameCompleted_C" null self))
      (`UserWidget.AddToViewport` _returnvalue 9)
      (else
        (bind _returnvalue_2 (`|CreateWidget` "/Game/Assets/Blueprints/Widgets/Widget_LevelCompleted.Widget_LevelCompleted_C" null self))
        (`UserWidget.AddToViewport` _returnvalue_2 9)))
    (else
      (bind _returnvalue_3 (`|CreateWidget` "/Game/Assets/Blueprints/Widgets/Widget_GameOver.Widget_GameOver_C" null self))
      (`UserWidget.AddToViewport` _returnvalue_3 9)))
  (`self.SetInputMode` "NewEnumerator0"))

(event `CollectedPowerPickup`
  ;[1 1 1] For Each Living Enemy, They Can Now Die And They Are Running From The Player
  (for _array_element (`self.EnemiesList`)
    (if (`/Game/Assets/Blueprints/MasterCharacter.IsCharacterAlive?` _array_element)
      (set `/Game/Assets/Blueprints/Base_Enemy.RunningFromPlayer?` true _array_element)
      (set `/Game/Assets/Blueprints/MasterCharacter.CanCharacterDie?` true _array_element)
      (`self.ChangeColors` _array_element (struct :`R` 1.0 :`G` 1.0 :`B` 1.0 :`A` 1.0))))
  ;[1 0 0] When Power Pickup Time Ends, Return All Living Enemies To Normal State
  (`KismetSystemLibrary.RetriggerableDelay` (`self.PowerPelletDuration`))
  (for _array_element_2 (`self.EnemiesList`)
    (if (`/Game/Assets/Blueprints/MasterCharacter.IsCharacterAlive?` _array_element_2)
      (set `/Game/Assets/Blueprints/Base_Enemy.RunningFromPlayer?` false _array_element_2)
      (set `/Game/Assets/Blueprints/Base_Enemy.ChasingPlayer?` true _array_element_2)
      (set `/Game/Assets/Blueprints/MasterCharacter.CanCharacterDie?` false _array_element_2)
      (`self.ChangeColors` _array_element_2 (`/Game/Assets/Blueprints/MasterCharacter.Color` _array_element_2)))))

(event `Key|LeftShift`
  (params (Key :type "Key Structure"))
  (bind _particlesystem (`self.ParticleSystem`))
  (:`Pressed`
    (`self.ChangeMaxSpeed` 2000.0 900.0)
    (`ActorComponent.Activate` _particlesystem false))
  (:`Released`
    (`self.ChangeMaxSpeed` 600.0 600.0)
    (`ActorComponent.Deactivate` _particlesystem)))

(fn `ChangeMaxSpeed`
  (params (MaxWalkSpeed :type "Float (double-precision)") (JumpZVelocity :type "Float (double-precision)"))
  (bind _charactermovement (`self.CharacterMovement`))
  (set `CharacterMovementComponent.MaxWalkSpeed` MaxWalkSpeed _charactermovement)
  (set `CharacterMovementComponent.JumpZVelocity` JumpZVelocity _charactermovement))

(fn `CompletionCheck`
  (bind _allcollectibleslist (`self.AllCollectiblesList`))
  (`KismetArrayLibrary.Array_Remove` _allcollectibleslist)
  (if (<= (`KismetArrayLibrary.Array_Length` _allcollectibleslist) 0)
    (`self.LevelEnd`)))

(fn `IncreaseCount`
  (params (PickupType :type "/Game/Assets/Blueprints/Enums/PickupType Enum" :default "NewEnumerator0"))
  (`/Engine/EditorBlueprintResources/StandardMacros.IncrementInt` (`self.PickedUpAmount`)
    (:`  `
      (`GameplayStatics.PlaySound2D` (select `/Game/Assets/Blueprints/Enums/PickupType` PickupType :`NewEnumerator0` "/Game/Assets/Blueprints/Audio/DotCollected.DotCollected" :`NewEnumerator1` "/Game/Assets/Blueprints/Audio/PowerPickup.PowerPickup" :!type "SoundBase Object Reference") 0.5 1.0 0.0 null null)
      (`self.CompletionCheck`))))

(fn `SetInputMode`
  (params (Selection :type "/Game/Assets/Blueprints/Enums/InputMode Enum" :default "NewEnumerator0"))
  (bind _playercontroller (`self.PlayerController`))
  (bind _playercontroller_2 (`self.PlayerController`))
  (switch `/Game/Assets/Blueprints/Enums/InputMode` Selection
    (:`NewEnumerator0`
      (`WidgetBlueprintLibrary.SetInputMode_UIOnlyEx` _playercontroller (`self.HUD`))
      (set `PlayerController.bShowMouseCursor` true _playercontroller))
    (:`NewEnumerator1`
      (`WidgetBlueprintLibrary.SetInputMode_GameOnly` _playercontroller_2)
      (set `PlayerController.bShowMouseCursor` false _playercontroller_2))))

(fn `UserConstructionScript`
  (`parent.UserConstructionScript`))